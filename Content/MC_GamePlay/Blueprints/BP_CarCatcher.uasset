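; BP_CarCatcher is an overlap-triggered actor that catches cars leaving the track and disqualifies their players.
; On begin overlap, only the authority resolves the overlapping actor's instigator controller to an RT_PlayerController and its RT_PlayerState.
; It logs the player number, then calls PlayerDisqualified on the RT_GameState with an off-track violation reason.
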(event `self.ReceiveActorBeginOverlap`
  (params (OtherActor :type "Actor Object Reference"))
  (`/Engine/EditorBlueprintResources/ActorMacros.Switch Has Authority`
    (:`Authority`
      (bind _asrt_player_controller (cast `/Game/MC_GamePlay/RT_PlayerController` (`self.GetInstigatorController` OtherActor)))
      (bind _asrt_player_state (cast `/Game/MC_GamePlay/RT_PlayerState` (`Controller.PlayerState` _asrt_player_controller)))
      (`KismetSystemLibrary.PrintString` (`KismetStringLibrary.Concat_StrStr` "Player Number:  " (`KismetStringLibrary.Conv_IntToString` (`/Game/MC_GamePlay/RT_PlayerState.PlayerNumber` _asrt_player_state)) " - Off Track") false)
      (`/Game/MC_GamePlay/RT_GameState.PlayerDisqualified` (cast `/Game/MC_GamePlay/RT_GameState` (`GameplayStatics.GetGameState`) :!pure true) _asrt_player_state "Off Track Violation"))))

(fn `UserConstructionScript`)