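; Lobby start-light prop that plays an endless countdown-style light sequence.
; BeginPlay starts a looping 0.4-second timer that calls GoToNextRow by function name.
; GoToNextRow switches on the Row enum, showing one light component at a time through five yellows, green and red, then blanks all and repeats.
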(event `self.ReceiveBeginPlay`
  (bind _countdownlightstimerhandle (`self.CountdownLightsTimerHandle`))
  (set `self.Row` "NewEnumerator7")
  (if (`KismetSystemLibrary.K2_IsValidTimerHandle` _countdownlightstimerhandle)
    (`KismetSystemLibrary.K2_ClearAndInvalidateTimerHandle` _countdownlightstimerhandle))
  (bind _returnvalue (`KismetSystemLibrary.K2_SetTimer` null "GoToNextRow" 0.4 true))
  (set `self.CountdownLightsTimerHandle` _returnvalue))

(fn `GoToNextRow`
  (switch `/Game/MC_GamePlay/Blueprints/StartLightEnum` (`self.Row`)
    (:`NewEnumerator7`
      (`SceneComponent.SetVisibility` (`self.Yellow1`) false true)
      (`SceneComponent.SetVisibility` (`self.Yellow2`) false true)
      (`SceneComponent.SetVisibility` (`self.Yellow3`) false true)
      (`SceneComponent.SetVisibility` (`self.Yellow4`) false true)
      (`SceneComponent.SetVisibility` (`self.Yellow5`) false true)
      (`SceneComponent.SetVisibility` (`self.Green6`) false true)
      (`SceneComponent.SetVisibility` (`self.Red7`) false true)
      (set `self.Row` "NewEnumerator0"))
    (:`NewEnumerator0`
      (`SceneComponent.SetVisibility` (`self.Yellow1`) true true)
      (`SceneComponent.SetVisibility` (`self.Yellow2`) false true)
      (`SceneComponent.SetVisibility` (`self.Yellow3`) false true)
      (`SceneComponent.SetVisibility` (`self.Yellow4`) false true)
      (`SceneComponent.SetVisibility` (`self.Yellow5`) false true)
      (`SceneComponent.SetVisibility` (`self.Green6`) false true)
      (`SceneComponent.SetVisibility` (`self.Red7`) false true)
      (set `self.Row` "NewEnumerator1"))
    (:`NewEnumerator1`
      (`SceneComponent.SetVisibility` (`self.Yellow1`) false true)
      (`SceneComponent.SetVisibility` (`self.Yellow2`) true true)
      (`SceneComponent.SetVisibility` (`self.Yellow3`) false true)
      (`SceneComponent.SetVisibility` (`self.Yellow4`) false true)
      (`SceneComponent.SetVisibility` (`self.Yellow5`) false true)
      (`SceneComponent.SetVisibility` (`self.Green6`) false true)
      (`SceneComponent.SetVisibility` (`self.Red7`) false true)
      (set `self.Row` "NewEnumerator2"))
    (:`NewEnumerator2`
      (`SceneComponent.SetVisibility` (`self.Yellow1`) false true)
      (`SceneComponent.SetVisibility` (`self.Yellow2`) false true)
      (`SceneComponent.SetVisibility` (`self.Yellow3`) true true)
      (`SceneComponent.SetVisibility` (`self.Yellow4`) false true)
      (`SceneComponent.SetVisibility` (`self.Yellow5`) false true)
      (`SceneComponent.SetVisibility` (`self.Green6`) false true)
      (`SceneComponent.SetVisibility` (`self.Red7`) false true)
      (set `self.Row` "NewEnumerator3"))
    (:`NewEnumerator3`
      (`SceneComponent.SetVisibility` (`self.Yellow1`) false true)
      (`SceneComponent.SetVisibility` (`self.Yellow2`) false true)
      (`SceneComponent.SetVisibility` (`self.Yellow3`) false true)
      (`SceneComponent.SetVisibility` (`self.Yellow4`) true true)
      (`SceneComponent.SetVisibility` (`self.Yellow5`) false true)
      (`SceneComponent.SetVisibility` (`self.Green6`) false true)
      (`SceneComponent.SetVisibility` (`self.Red7`) false true)
      (set `self.Row` "NewEnumerator4"))
    (:`NewEnumerator4`
      (`SceneComponent.SetVisibility` (`self.Yellow1`) false true)
      (`SceneComponent.SetVisibility` (`self.Yellow2`) false true)
      (`SceneComponent.SetVisibility` (`self.Yellow3`) false true)
      (`SceneComponent.SetVisibility` (`self.Yellow4`) false true)
      (`SceneComponent.SetVisibility` (`self.Yellow5`) true true)
      (`SceneComponent.SetVisibility` (`self.Green6`) false true)
      (`SceneComponent.SetVisibility` (`self.Red7`) false true)
      (set `self.Row` "NewEnumerator5"))
    (:`NewEnumerator5`
      (`SceneComponent.SetVisibility` (`self.Yellow1`) false true)
      (`SceneComponent.SetVisibility` (`self.Yellow2`) false true)
      (`SceneComponent.SetVisibility` (`self.Yellow3`) false true)
      (`SceneComponent.SetVisibility` (`self.Yellow4`) false true)
      (`SceneComponent.SetVisibility` (`self.Yellow5`) false true)
      (`SceneComponent.SetVisibility` (`self.Green6`) true true)
      (`SceneComponent.SetVisibility` (`self.Red7`) false true)
      (set `self.Row` "NewEnumerator6"))
    (:`NewEnumerator6`
      (`SceneComponent.SetVisibility` (`self.Yellow1`) false true)
      (`SceneComponent.SetVisibility` (`self.Yellow2`) false true)
      (`SceneComponent.SetVisibility` (`self.Yellow3`) false true)
      (`SceneComponent.SetVisibility` (`self.Yellow4`) false true)
      (`SceneComponent.SetVisibility` (`self.Yellow5`) false true)
      (`SceneComponent.SetVisibility` (`self.Green6`) false true)
      (`SceneComponent.SetVisibility` (`self.Red7`) true true)
      (set `self.Row` "NewEnumerator7"))))

(fn `UserConstructionScript`)