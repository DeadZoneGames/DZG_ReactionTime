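; BP_FinishLine is a finish line trigger that reports when a player crosses it.
; On the server only, an overlap on its collision component resolves the overlapping actor's instigator controller to an RT_PlayerController and its RT_PlayerState.
; It passes that state to RT_GameState's PlayerCrossesFinishLIne, printing the player number or cast failures as debug messages.
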(event `self.CollisionComponent.OnComponentBeginOverlap`
  (params (OverlappedComponent :type "PrimitiveComponent Object Reference") (OtherActor :type "Actor Object Reference") (OtherComp :type "PrimitiveComponent Object Reference") (OtherBodyIndex :type Integer) (bFromSweep :type Boolean) (SweepResult :type "HitResult Structure (by ref)"))
  (`/Engine/EditorBlueprintResources/ActorMacros.Switch Has Authority`
    (:`Authority`
      (bind _asrt_player_controller (cast `/Game/MC_GamePlay/RT_PlayerController` (`self.GetInstigatorController` OtherActor))
        (:`then`
          (bind _asrt_player_state (cast `/Game/MC_GamePlay/RT_PlayerState` (`Controller.PlayerState` _asrt_player_controller))
            (:`then`
              (`KismetSystemLibrary.PrintString` (`KismetStringLibrary.Concat_StrStr` "FINISH LINE! Player Number: " (`KismetStringLibrary.Conv_IntToString` (`/Game/MC_GamePlay/RT_PlayerState.PlayerNumber` _asrt_player_state))) true true (struct :`R` 0.003728 :`B` 0.65625 :`A` 1.0) 5.0)
              (`/Game/MC_GamePlay/RT_GameState.PlayerCrossesFinishLIne` (cast `/Game/MC_GamePlay/RT_GameState` (`GameplayStatics.GetGameState`) :!pure true) _asrt_player_state))
            (:`CastFailed`
              (`KismetSystemLibrary.PrintString` "FINISH LINE: CAST TO RT_PlayerState FAILED!" false))))
        (:`CastFailed`
          (`KismetSystemLibrary.PrintString` "FINISH LINE: CAST TO RT_PlayerController FAILED!" false))))))

(fn `UserConstructionScript`)