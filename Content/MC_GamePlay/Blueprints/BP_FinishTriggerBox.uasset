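; BP_FinishTriggerBox is a trigger volume that marks the finish of a race for RT_TopFuel1 vehicles.
; On component overlap, only the server casts the overlapping actor to RT_TopFuel1 and gets its RT_PlayerState.
; It prints the player number as debug text, then passes that player state to RT_GameState to record the player's finish time.
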(event `self.CollisionComponent.OnComponentBeginOverlap`
  (params (OverlappedComponent :type "PrimitiveComponent Object Reference") (OtherActor :type "Actor Object Reference") (OtherComp :type "PrimitiveComponent Object Reference") (OtherBodyIndex :type Integer) (bFromSweep :type Boolean) (SweepResult :type "HitResult Structure (by ref)"))
  (`/Engine/EditorBlueprintResources/ActorMacros.Switch Has Authority`
    (:`Authority`
      (bind _asrt_top_fuel_1 (cast `/Game/MC_VehicleBP/RT_TopFuel1` OtherActor))
      (bind _asrt_player_state (cast `/Game/MC_GamePlay/RT_PlayerState` (`Pawn.PlayerState` _asrt_top_fuel_1)))
      (`KismetSystemLibrary.PrintString` (`KismetStringLibrary.Concat_StrStr` "Trigger Box Player Number:  " (`KismetStringLibrary.Conv_IntToString` (`/Game/MC_GamePlay/RT_PlayerState.PlayerNumber` _asrt_player_state))) true true (struct :`G` 0.66 :`B` 1.0 :`A` 1.0) 30.0)
      (bind _asrt_game_state (cast `/Game/MC_GamePlay/RT_GameState` (`GameplayStatics.GetGameState`)))
      (`/Game/MC_GamePlay/RT_GameState.RecordPlayersFinishTime` _asrt_game_state _asrt_player_state))))

(fn `UserConstructionScript`)